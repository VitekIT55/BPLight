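; A light actor that blinks its PointLight on and off after play begins.
; BeginPlay runs a self-looping DoN, Delay and FlipFlop chain that alternates LightOn and LightOff, with SetDoN capping the toggle count and SetDuration setting the interval.
; The construction script sets initial visibility from DefLight; a DefaultLight function does the same but is not called in these graphs.
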(event `self.ReceiveBeginPlay`
  (`/Engine/EditorBlueprintResources/StandardMacros.Do N` (`self.Set Do N`) :!label _label
    (:`Exit`
      (`KismetSystemLibrary.Delay` (`self.Set Duration`))
      (`/Engine/EditorBlueprintResources/StandardMacros.FlipFlop`
        (:`A`
          (`self.LightOn`)
          (goto _label))
        (:`B`
          (`self.LightOff`)
          (goto _label))))))

(fn `DefaultLight`
  (`SceneComponent.SetVisibility` (`self.PointLight`) (`self.DefLight`) false))

(fn `LightOff`
  (`SceneComponent.SetVisibility` (`self.PointLight`) false false))

(fn `LightOn`
  (`SceneComponent.SetVisibility` (`self.PointLight`) true false))

(fn `UserConstructionScript`
  (`SceneComponent.SetVisibility` (`self.PointLight`) (`self.DefLight`) false))